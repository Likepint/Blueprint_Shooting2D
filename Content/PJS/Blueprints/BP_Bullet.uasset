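; BP_Bullet is a projectile actor that destroys enemies and awards score.
; Each tick it moves along its forward vector at its Speed, scaled by delta time, without sweeping.
; On overlapping a BP_Enemy, it adds a point through BP_GameMode, updates the high score, then destroys both the enemy and itself.
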(event Collision|EventActorBeginOverlap
  (params (OtherActor :type Actor%20Object%20Reference))
  (bind _asbp_enemy (Utilities|Casting|CastToBP_Enemy OtherActor))
  (bind _asbp_game_mode (Utilities|Casting|CastToBP_GameMode (Game|GetGameMode)))
  (Default|AddCurrentScore _asbp_game_mode 1)
  (Default|UpdateHighScore _asbp_game_mode)
  (Actor|DestroyActor _asbp_enemy)
  (Actor|DestroyActor))

(event EventTick
  (params (DeltaSeconds :type Float%20%28single-precision%29))
  ;[0.15 0.15 0.15 0.5] 살아있는 동안 앞으로 이동 구현
  (Transformation|SetActorLocation (+ (Transformation|GetActorLocation) (* (* (Transformation|GetActorForwardVector) (Variables|Default|GetSpeed)) (Utilities|Time|GetWorldDeltaSeconds))) false false))

(fn ConstructionScript)