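; BP_GameMode is a game mode that shows the main UI and tracks the current score and a persistent high score.
; On BeginPlay it creates WBP_MainUI, then loads or creates a BP_ScoreData save in the "Score" slot to seed HighScore.
; AddCurrentScore accumulates points, and UpdateHighScore saves CurrentScore when it beats the record.
; A UI visibility toggle based on player pawn validity is present but unconnected.
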(event EventBeginPlay
  (bind _returnvalue (UserInterface|CreateWidget "/Game/PJS/UI/WBP_MainUI.WBP_MainUI_C"))
  (UserInterface|Viewport|AddtoViewport _returnvalue 0)
  (bind _returnvalue_2 (SaveGame|DoesSaveGameExist "Score"))
  (if _returnvalue_2
    (bind _returnvalue_3 (SaveGame|LoadGamefromSlot "Score"))
    (bind _asbp_score_data (Utilities|Casting|CastToBP_ScoreData _returnvalue_3))
    (bind _output_get (Variables|Default|SetSaveRef _asbp_score_data))
    (Variables|Default|SetHighScore (Variables|/Game/PJS/SaveData/BP_ScoreData.BP_ScoreData_C|GetBestScore _output_get))
    (else
      (bind _returnvalue_4 (SaveGame|CreateSaveGameObject "/Game/PJS/SaveData/BP_ScoreData.BP_ScoreData_C"))
      (bind _output_get_2 (Variables|Default|SetSaveRef _returnvalue_4))
      (Variables|Default|SetHighScore (Variables|/Game/PJS/SaveData/BP_ScoreData.BP_ScoreData_C|GetBestScore _output_get_2)))))

(event EventTick
  (params (DeltaSeconds :type Float%20%28single-precision%29)))

(fn ConstructionScript)

(fn AddCurrentScore
  (params (Point :type Integer))
  (Variables|Default|SetCurrentScore (+ Point (Variables|Default|GetCurrentScore))))

(fn UpdateHighScore
  (bind _saveref (Variables|Default|GetSaveRef))
  (if (> (Variables|Default|GetCurrentScore) (Variables|Default|GetHighScore))
    (bind _output_get (Variables|Default|SetHighScore (Variables|Default|GetCurrentScore)))
    (Variables|/Game/PJS/SaveData/BP_ScoreData.BP_ScoreData_C|SetBestScore _saveref _output_get)
    (SaveGame|SaveGametoSlot _saveref "Score")))