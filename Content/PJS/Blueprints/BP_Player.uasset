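; Player actor that moves on the Y/Z plane and fires bullets, with game-only input and a hidden cursor.
; Horizontal and Vertical axis events share one normalized direction, applied by Translation as frame-rate-independent movement without sweep.
; Fire spawns BP_Bullet at FirePosition.
; Tick saves the location, then snaps back to it while overlapping BP_DeadZone; disconnected earlier movement experiments remain in the graph.
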(event Collision|EventActorBeginOverlap
  (params (OtherActor :type Actor%20Object%20Reference))
  (Utilities|Casting|CastToBP_DeadZone OtherActor)
  (Variables|Default|SetbFixed true))

(event EventTick
  (params (DeltaSeconds :type Float%20%28single-precision%29))
  (if (Variables|Default|GetbFixed)
    (Transformation|SetActorLocation (Variables|Default|GetLocation) false false)
    (else
      (Variables|Default|SetLocation (Transformation|GetActorLocation)))))

(event Collision|EventActorEndOverlap
  (params (OtherActor :type Actor%20Object%20Reference))
  (Utilities|Casting|CastToBP_DeadZone OtherActor)
  (Variables|Default|SetbFixed false))

(event EventBeginPlay
  (bind _returnvalue (Game|GetPlayerController 0))
  (Variables|/Script/Engine.PlayerController|SetbShowMouseCursor _returnvalue false)
  (Input|SetInputModeGameOnly _returnvalue false))

(event Input|ActionEvents|InputActionFire
  (params (Key :type Key%20Structure :default "None"))
  (:Pressed
    (Game|SpawnActorfromClass "/Game/PJS/Blueprints/BP_Bullet.BP_Bullet_C" (Transformation|GetWorldTransform (Variables|Default|GetFirePosition)) "Undefined" "MultiplyWithRoot" 0 0)))

(event Input|AxisEvents|InputAxisHorizontal
  (params (AxisValue :type Float%20%28single-precision%29))
  ;[0.15 0.15 0.15 0.5] V ( 방향 * 속력 )
  (CallFunction|Translation (Math|Vector|Normalize (Math|Vector|MakeVector 0.0 AxisValue (stale Input|AxisEvents|InputAxisVertical AxisValue))) (Variables|Default|GetSpeed) (Utilities|Time|GetWorldDeltaSeconds)))

(event Input|AxisEvents|InputAxisVertical
  (params (AxisValue :type Float%20%28single-precision%29))
  ;[0.15 0.15 0.15 0.5] V ( 방향 * 속력 )
  (CallFunction|Translation (Math|Vector|Normalize (Math|Vector|MakeVector 0.0 (stale Input|AxisEvents|InputAxisHorizontal AxisValue) AxisValue)) (Variables|Default|GetSpeed) (Utilities|Time|GetWorldDeltaSeconds)))

(fn ConstructionScript)

(fn Translation
  (params (NormalizedDirection :type Vector) (Speed :type Float%20%28double-precision%29) (WorldDeltaSeconds :type Float%20%28double-precision%29))
  (Transformation|SetActorLocation (+ (* NormalizedDirection Speed WorldDeltaSeconds) (Transformation|GetActorLocation)) false false))