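; BP_Tail is an actor that follows a Target, defaulting to the player pawn, by moving straight toward it.
; BeginPlay fills an unset Target with player 0's pawn cast to BP_Player.
; Each Tick passes the normalized direction, Speed and delta seconds to Translation, which offsets the location without sweep or stopping distance.
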(event EventBeginPlay
  ;[0.15 0.15 0.15 0.5] Needs : Speed, Target
  ;;[0.15 0.15 0.15 0.5] Target = player
  (Utilities|IsValid (Variables|Default|GetTarget)
    (:Is%20Not%20Valid
      (bind _asbp_player (Utilities|Casting|CastToBP_Player (Game|Player|GetPlayerPawn 0)))
      (Utilities|IsValid _asbp_player
        (:Is%20Valid
          (Variables|Default|SetTarget _asbp_player))))))

(event EventTick
  (params (DeltaSeconds :type Float%20%28single-precision%29))
  ;[0.15 0.15 0.15 0.5] Needs : Speed, Target
  (CallFunction|Translation (Math|Vector|Normalize (- (Transformation|GetActorLocation (Variables|Default|GetTarget)) (Transformation|GetActorLocation))) (Variables|Default|GetSpeed) (Utilities|Time|GetWorldDeltaSeconds)))

(fn ConstructionScript)

(fn Translation
  (params (NormalizedDirection :type Vector) (Speed :type Float%20%28double-precision%29) (WorldDeltaSeconds :type Float%20%28double-precision%29))
  (Transformation|SetActorLocation (+ (* NormalizedDirection Speed WorldDeltaSeconds) (Transformation|GetActorLocation)) false false))